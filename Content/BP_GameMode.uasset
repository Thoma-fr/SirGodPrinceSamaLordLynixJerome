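; Game mode that provides debug keyboard shortcuts to save and load game state.
; It enables input on BeginPlay, then P creates a SaveState object, fills it from the first player controller and writes it to a fixed save slot on success.
; O loads that slot, casts it to SaveState and has it apply its data to the player controller.
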(event EventTick
  (params (DeltaSeconds :type Float%20%28single-precision%29)))

(event EventBeginPlay
  (Input|EnableInput 0))

(event Input|KeyboardEvents|P
  (params (Key :type Key%20Structure :default "None"))
  (:Pressed
    (Development|PrintString "Hello")
    (bind _returnvalue (SaveGame|CreateSaveGameObject "/Game/SaveState.SaveState_C"))
    (bind _success (Default|SaveData _returnvalue (Game|GetPlayerController 0)))
    (if _success
      (SaveGame|SaveGametoSlot _returnvalue "MaGrosseSave")
      (Development|PrintString "la bonne save"))))

(event Input|KeyboardEvents|O
  (params (Key :type Key%20Structure :default "None"))
  (:Pressed
    (bind _returnvalue (SaveGame|LoadGamefromSlot "MaGrosseSave"))
    (bind _assave_state (Utilities|Casting|CastToSaveState _returnvalue))
    (Default|LoadData _assave_state (Game|GetPlayerController 0))))

(fn ConstructionScript)